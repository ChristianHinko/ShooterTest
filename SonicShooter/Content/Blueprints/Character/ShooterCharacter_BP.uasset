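; Shooter character Blueprint whose only active logic is a test hotkey for possessing another pawn.
; Pressing P runs a long, debug-drawn object line trace from the character's location along its controller's forward vector.
; If the hit actor is a Pawn, the ServerPossess event has the current controller possess it.
; BeginPlay, overlap, Tick and the construction script are empty.
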(event Custom|ServerPossess
  (params (NewParam :type Pawn%20Object%20Reference))
  ;[1 1 1] Testing
  (Pawn|Possess (Pawn|GetController) NewParam))

(event EventBeginPlay)

(event Collision|EventActorBeginOverlap
  (params (OtherActor :type Actor%20Object%20Reference)))

(event EventTick
  (params (DeltaSeconds :type Float%20%28single-precision%29)))

(event Input|KeyboardEvents|P
  (params (Key :type Key%20Structure))
  (bind _returnvalue (Transformation|GetActorLocation))
  ;[1 1 1] Testing
  (:Pressed
    (bind _outhit (Collision|LineTraceForObjects _returnvalue (+ _returnvalue (* (Transformation|GetActorForwardVector (Pawn|GetController)) 1e+05)) (Utilities|Array|MakeArray "ObjectTypeQuery1" "ObjectTypeQuery2" "ObjectTypeQuery3" "ObjectTypeQuery4") false 0 "ForDuration"))
    (bind _aspawn (Utilities|Casting|CastToPawn (.HitActor (Collision|BreakHitResult _outhit))))
    (CallFunction|ServerPossess _aspawn)))

(fn ConstructionScript)