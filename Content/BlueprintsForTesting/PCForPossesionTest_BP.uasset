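; Test player controller for switching pawn possession through debug keys.
; Delete alternates between two PawnInfos entries, and a server event sets it as pending, spawns that pawn and possesses it.
; Tab sphere-traces forward from the controlled pawn to possess the pawn it hits, while 1 picks a random pawn in the level.
; Both route through a second server event that possesses the target and prints its name.
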(event Custom|Server_Posses
  (params (NewParam :type Pawn%20Object%20Reference))
  (Pawn|Possess NewParam)
  (Development|PrintString (Utilities|String|Append "Possessed: " (Utilities|GetDisplayName NewParam))))

(event Custom|Server_SetPendingPawnInfo
  (params (NewPawnInfo :type Pawn%20Info%20Structure))
  (Class|GTPlayerController|SetPendingPawnInfo NewPawnInfo)
  (bind _returnvalue (Class|GTPlayerController|SpawnPawnfromPendingInfo))
  (Pawn|Possess _returnvalue))

(event Input|KeyboardEvents|Delete
  (params (Key :type Key%20Structure :default "None"))
  (:Pressed
    (Utilities|FlowControl|FlipFlop
      (:A
        (CallFunction|ServerSetPendingPawnInfo (Utilities|Array|Get(acopy) (Variables|Default|GetPawnInfos) 1)))
      (:B
        (CallFunction|ServerSetPendingPawnInfo (Utilities|Array|Get(acopy) (Variables|Default|GetPawnInfos)))))))

(event Input|KeyboardEvents|Tab
  (params (Key :type Key%20Structure :default "None"))
  (bind _returnvalue (Pawn|GetControlledPawn))
  (bind _returnvalue_2 (Transformation|GetActorLocation _returnvalue))
  (:Pressed
    (bind (_outhit _returnvalue_3) (Collision|SphereTraceForObjects _returnvalue_2 (+ _returnvalue_2 (* (Transformation|GetActorForwardVector _returnvalue) 1e+04)) 5e+01 (Utilities|Array|MakeArray "ObjectTypeQuery1" "ObjectTypeQuery2" "ObjectTypeQuery3" "ObjectTypeQuery4" "ObjectTypeQuery5" "ObjectTypeQuery6") false (Utilities|Array|MakeArray _returnvalue) "ForDuration"))
    (if _returnvalue_3
      (bind _aspawn (Utilities|Casting|CastToPawn (.HitActor (Collision|BreakHitResult _outhit))))
      (CallFunction|ServerPosses _aspawn))))

(event Input|KeyboardEvents|1
  (params (Key :type Key%20Structure :default "None"))
  (:Pressed
    (bind _outactors (Actor|GetAllActorsOfClass "/Script/Engine.Pawn"))
    (CallFunction|ServerPosses (Utilities|Array|Get(acopy) _outactors (Math|Random|RandomIntegerinRange 0 (- (Utilities|Array|Length _outactors) 1))))))

(fn ConstructionScript)