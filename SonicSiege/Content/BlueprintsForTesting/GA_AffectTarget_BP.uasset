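; GA_AffectTarget_BP is a test Gameplay Ability that applies a gameplay effect to the first target in front of the avatar.
; On activation it commits, then runs a long, debug-drawn sphere trace along the avatar's forward vector, ignoring the avatar.
; If the hit actor has an Ability System Component, it applies GE_CharacterLargeDec_BP to it via actor target data.
; The ability ends immediately in every case.
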(event Ability|EventActivateAbility
  (bind _returnvalue (Ability|GetAvatarActorfromActorInfo))
  (bind _returnvalue_2 (Transformation|GetActorLocation _returnvalue))
  (Ability|CommitAbility)
  (bind (_outhit _returnvalue_3) (Collision|SphereTraceForObjects _returnvalue_2 (+ _returnvalue_2 (* (Transformation|GetActorForwardVector _returnvalue) 1e+04)) 5e+01 (Utilities|Array|MakeArray "ObjectTypeQuery1" "ObjectTypeQuery2" "ObjectTypeQuery3" "ObjectTypeQuery4" "ObjectTypeQuery5" "ObjectTypeQuery6") false (Utilities|Array|MakeArray _returnvalue) "ForDuration" true "(R=1.000000,G=0.136000,B=0.000000,A=1.000000)" "(R=0.000000,G=0.368750,B=1.000000,A=1.000000)"))
  (if _returnvalue_3
    (Utilities|IsValid (Ability|GetAbilitySystemComponent (.HitActor (Collision|BreakHitResult _outhit)))
      (:Is%20Valid
        (GameplayEffects|ApplyGameplayEffectToTarget (Ability|TargetData|AbilityTargetDatafromActor (.HitActor (Collision|BreakHitResult _outhit))) "/Game/BlueprintsForTesting/GE_CharacterLargeDec_BP.GE_CharacterLargeDec_BP_C" 1 1)
        (Ability|EndAbility))
      (:Is%20Not%20Valid
        (Ability|EndAbility)))
    (else
      (Ability|EndAbility))))

(event Ability|EventOnEndAbility
  (params (bWasCancelled :type Boolean)))